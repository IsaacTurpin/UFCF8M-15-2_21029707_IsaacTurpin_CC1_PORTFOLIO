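; Light actor that flickers endlessly from BeginPlay, with a flicker sound played once at its location on start.
; A self-calling Flicker event chains randomized delays into two off-on blinks per cycle, with short dark gaps between longer lit periods.
; TurnOff and TurnOn toggle the SpotLight's visibility and swap the bulb mesh material between black unlit and basic shape to match.
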(event `Flicker`
  (`KismetSystemLibrary.Delay` (`KismetMathLibrary.RandomFloatInRange` 0.8 1.4) :!label _label)
  (`self.Turn Off`)
  (`KismetSystemLibrary.Delay` (`KismetMathLibrary.RandomFloatInRange` 0.1 0.3))
  (`self.Turn On`)
  (`KismetSystemLibrary.Delay` (`KismetMathLibrary.RandomFloatInRange` 1.0 1.5))
  (`self.Turn Off`)
  (`KismetSystemLibrary.Delay` (`KismetMathLibrary.RandomFloatInRange` 0.3 0.7))
  (`self.Turn On`)
  (`self.Flicker`))

(event `self.ReceiveBeginPlay`
  (`GameplayStatics.PlaySoundAtLocation` "/Game/143915__scotchio__flickeringlight_Cue.143915__scotchio__flickeringlight_Cue" (`self.K2_GetActorLocation`) (struct) 1.0 1.0 0.0 null null null null)
  (goto _label))

(event `Turn Off`
  (`PrimitiveComponent.SetMaterial` (`self.Bulb SM`) 0 "/Engine/EngineDebugMaterials/BlackUnlitMaterial.BlackUnlitMaterial")
  (`SceneComponent.SetVisibility` (`self.SpotLight`) false false))

(event `Turn On`
  (`PrimitiveComponent.SetMaterial` (`self.Bulb SM`) 0 "/Engine/BasicShapes/BasicShapeMaterial.BasicShapeMaterial")
  (`SceneComponent.SetVisibility` (`self.SpotLight`) true false))

(fn `UserConstructionScript`)