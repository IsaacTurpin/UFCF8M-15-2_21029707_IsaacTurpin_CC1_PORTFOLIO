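; Flashing alarm siren actor that plays a base alarm sound at its location on BeginPlay and blinks continuously.
; Flicker alternates TurnOff and TurnOn on half-second delays, then calls itself to repeat indefinitely.
; Each toggle swaps the bulb mesh between a base and red material and hides or shows the spotlight.
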(event `Flicker`
  (`KismetSystemLibrary.Delay` 0.5 :!label _label)
  (`self.Turn Off`)
  (`KismetSystemLibrary.Delay` 0.5)
  (`self.Turn On`)
  (`KismetSystemLibrary.Delay` 0.5)
  (`self.Turn Off`)
  (`KismetSystemLibrary.Delay` 0.5)
  (`self.Turn On`)
  (`self.Flicker`))

(event `self.ReceiveBeginPlay`
  (`GameplayStatics.PlaySoundAtLocation` "/Game/388878__deleted-user-7313090__base-alarm_Cue.388878__deleted-user-7313090__base-alarm_Cue" (`self.K2_GetActorLocation`) (struct) 1.0 1.0 0.0 null null null null)
  (goto _label))

(event `Turn Off`
  (`PrimitiveComponent.SetMaterial` (`self.BulbSM`) 0 "/AnimationSharing/AnimSharingBase.AnimSharingBase")
  (`SceneComponent.SetVisibility` (`self.SpotLight`) false false))

(event `Turn On`
  (`PrimitiveComponent.SetMaterial` (`self.BulbSM`) 0 "/AnimationSharing/AnimSharingRed.AnimSharingRed")
  (`SceneComponent.SetVisibility` (`self.SpotLight`) true false))

(fn `UserConstructionScript`)