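; RiseCoinBP is a collectible coin that toggles linked rising platforms when the third-person character picks it up.
; On BeginPlay it caches every FloorRiseBP actor in an array.
; Trigger overlap adds to the character's items, plays a sound and destroys the coin, then sends TogglePlatformsMessage to cached platforms sharing its PlatformIndex.
; The destroy call runs before the platform loop in the same event.
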(event `self.ReceiveBeginPlay`
  (bind _outactors (`GameplayStatics.GetAllActorsOfClass` "/Game/FloorRiseBP.FloorRiseBP_C"))
  (for _array_element _outactors
    (`KismetArrayLibrary.Array_Add` (`self.Platform Array`) _array_element)))

(event `self.Trigger.OnComponentBeginOverlap`
  (params (OverlappedComponent :type "PrimitiveComponent Object Reference") (OtherActor :type "Actor Object Reference") (OtherComp :type "PrimitiveComponent Object Reference") (OtherBodyIndex :type Integer) (bFromSweep :type Boolean) (SweepResult :type "HitResult Structure (by ref)"))
  (bind _asbp_third_person_character (cast `/Game/ThirdPerson/Blueprints/BP_ThirdPersonCharacter` OtherActor))
  (`/Game/ThirdPerson/Blueprints/BP_ThirdPersonCharacter.AddItems` _asbp_third_person_character)
  (`self.CoinPlaySound`)
  (for _array_element (`self.Platform Array`)
    (if (== (`/Game/FloorRiseBP.Platform Index` _array_element) (`self.Platform Index`))
      (message `/Game/PlatformInterface.Toggle Platforms` _array_element))))

(event `CoinPlaySound`
  (`GameplayStatics.PlaySoundAtLocation` "/Game/StarterContent/Audio/Explosion_Cue.Explosion_Cue" (`self.K2_GetActorLocation`) (struct) 1.0 1.0 0.0 null null null null)
  (`self.K2_DestroyActor`))

(fn `UserConstructionScript`)